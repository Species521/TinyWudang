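; BP_Pavillion_small is a small pavilion building whose roof material changes while the player character is inside its trigger.
; On BeginPlay it swaps the roof's first material for a dynamic instance.
; Begin and end overlaps of BP_character_01 with the roof trigger play and reverse a Timeline, which drives a named scalar parameter on that instance, likely for a roof fade.
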(event `self.Pavillion_small_roof_trigger.OnComponentEndOverlap`
  (params (OverlappedComponent :type "PrimitiveComponent Object Reference") (OtherActor :type "Actor Object Reference") (OtherComp :type "PrimitiveComponent Object Reference") (OtherBodyIndex :type Integer))
  (cast `/Game/TopDown/Blueprints/BP_character_01` OtherActor)
  (bind (_direction _newtrack_0) (`Timeline|Timeline` :!via `Reverse` :!label _label)
    (:`Update`
      (`MaterialInstanceDynamic.SetScalarParameterValue` (`self.Dynamic Mat Reference`) (`self.Parameter Name`) _newtrack_0))))

(event `self.Pavillion_small_roof_trigger.OnComponentBeginOverlap`
  (params (OverlappedComponent :type "PrimitiveComponent Object Reference") (OtherActor :type "Actor Object Reference") (OtherComp :type "PrimitiveComponent Object Reference") (OtherBodyIndex :type Integer) (bFromSweep :type Boolean) (SweepResult :type "HitResult Structure (by ref)"))
  (cast `/Game/TopDown/Blueprints/BP_character_01` OtherActor)
  (goto _label))

(event `self.ReceiveBeginPlay`
  (bind _returnvalue (`KismetMaterialLibrary.CreateDynamicMaterialInstance` (`PrimitiveComponent.GetMaterial` (`self.pavillion_A_roof`) 0)))
  (bind _output_get (set `self.Dynamic Mat Reference` _returnvalue))
  (`PrimitiveComponent.SetMaterial` (`self.pavillion_A_roof`) 0 _output_get))

(fn `UserConstructionScript`)